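; BP_Dummy_follaw is a pawn that chases the first-person player and opens the Game_Over level when the player overlaps its Box.
; After a delay at BeginPlay, it starts a custom move event that runs AIMoveTo toward the player's current location.
; That event re-triggers itself on a delay to refresh the destination, printing debug strings and the move result.
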(event `AI move to`
  (bind _asbp_first_person_character (cast `/Game/FirstPerson/Blueprints/BP_FirstPersonCharacter` (`GameplayStatics.GetPlayerCharacter` 0)))
  (bind _output_get (set `self.FTC` _asbp_first_person_character))
  (bind _movementresult (`|AIMoveTo` self (`self.K2_GetActorLocation` _output_get) null)
    (:`then`
      (`KismetSystemLibrary.Delay` 3.0)
      (`KismetSystemLibrary.PrintString` "Hello")
      (`self.AI move to`))
    (:`OnSuccess`
      (`KismetSystemLibrary.PrintString` (`|GetEnumeratorNameAsString` _movementresult) :!label _label))
    (:`OnFail`
      (goto _label))))

(event `self.Box.OnComponentBeginOverlap`
  (params (OverlappedComponent :type "PrimitiveComponent Object Reference") (OtherActor :type "Actor Object Reference") (OtherComp :type "PrimitiveComponent Object Reference") (OtherBodyIndex :type Integer) (bFromSweep :type Boolean) (SweepResult :type "HitResult Structure (by ref)"))
  (cast `/Game/FirstPerson/Blueprints/BP_FirstPersonCharacter` OtherActor)
  (`GameplayStatics.OpenLevel` "Game_Over"))

(event `self.ReceiveBeginPlay`
  (`KismetSystemLibrary.Delay` 5.0)
  (`KismetSystemLibrary.PrintString` "walk'")
  (`self.AI move to`))

(fn `UserConstructionScript`)