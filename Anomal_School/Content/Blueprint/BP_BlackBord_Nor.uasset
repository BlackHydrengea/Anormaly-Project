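; Interactable blackboard actor that unlocks the current floor's exit in the Science Map and Computer Room levels.
; On IA_Interact it replaces itself with BP_BlackBord, then switches on the level name to destroy BP_worng_Door2 actors and spawn that level's transition or end door at BP_NextFloor_1's location.
; The box overlap only casts to the player character, so nothing in the graph gates the interaction by proximity.
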(event `self.Box.OnComponentBeginOverlap`
  (params (OverlappedComponent :type "PrimitiveComponent Object Reference") (OtherActor :type "Actor Object Reference") (OtherComp :type "PrimitiveComponent Object Reference") (OtherBodyIndex :type Integer) (bFromSweep :type Boolean) (SweepResult :type "HitResult Structure (by ref)"))
  (cast `/Game/FirstPerson/Blueprints/BP_FirstPersonCharacter` OtherActor))

(event `EnhancedInput|/Game/FirstPerson/Input/Actions/IA_Interact`
  (params (ActionValue :type Boolean) (ElapsedSeconds :type "Float (double-precision)") (TriggeredSeconds :type "Float (double-precision)") (InputAction :type "InputAction Object Reference" :default "/Game/FirstPerson/Input/Actions/IA_Interact.IA_Interact"))
  (:`Triggered`
    (`|SpawnActorFromClass` "/Game/Blueprint/BP_BlackBord.BP_BlackBord_C" (`self.GetTransform` self) "Undefined" "MultiplyWithRoot" null null)
    (`self.K2_DestroyActor` self)
    (bind _returnvalue (`GameplayStatics.GetCurrentLevelName` true))
    (switch `name` (`KismetStringLibrary.Conv_StringToName` _returnvalue)
      (:`Science_Map_1`
        (bind _outactors (`GameplayStatics.GetAllActorsOfClass` "/Game/Blueprint/BP_worng_Door2.BP_worng_Door2_C"))
        (`self.K2_DestroyActor` _outactors)
        (bind _returnvalue_2 (`GameplayStatics.GetActorOfClass` "/Game/Blueprint/BP_NextFloor_1.BP_NextFloor_1_C"))
        (`|SpawnActorFromClass` "/Game/FirstPerson/Maps/science_room/Lab_Door/Lab_1_to_2.Lab_1_to_2_C" (`KismetMathLibrary.Conv_VectorToTransform` (`self.K2_GetActorLocation` _returnvalue_2)) "Undefined" "MultiplyWithRoot" null null))
      (:`Science_Map_2`
        (bind _outactors_2 (`GameplayStatics.GetAllActorsOfClass` "/Game/Blueprint/BP_worng_Door2.BP_worng_Door2_C"))
        (`self.K2_DestroyActor` _outactors_2)
        (bind _returnvalue_3 (`GameplayStatics.GetActorOfClass` "/Game/Blueprint/BP_NextFloor_1.BP_NextFloor_1_C"))
        (`|SpawnActorFromClass` "/Game/FirstPerson/Maps/science_room/Lab_Door/Lab_2_to_3.Lab_2_to_3_C" (`KismetMathLibrary.Conv_VectorToTransform` (`self.K2_GetActorLocation` _returnvalue_3)) "Undefined" "MultiplyWithRoot" null null))
      (:`Science_Map_3`
        (bind _outactors_3 (`GameplayStatics.GetAllActorsOfClass` "/Game/Blueprint/BP_worng_Door2.BP_worng_Door2_C"))
        (`self.K2_DestroyActor` _outactors_3)
        (bind _returnvalue_4 (`GameplayStatics.GetActorOfClass` "/Game/Blueprint/BP_NextFloor_1.BP_NextFloor_1_C"))
        (`|SpawnActorFromClass` "/Game/Blueprint/Door/BP_EndDoor.BP_EndDoor_C" (`KismetMathLibrary.Conv_VectorToTransform` (`self.K2_GetActorLocation` _returnvalue_4)) "Undefined" "MultiplyWithRoot" null null))
      (:`Computer_Room_1`
        (bind _returnvalue_5 (`GameplayStatics.GetActorOfClass` "/Game/Blueprint/BP_worng_Door2.BP_worng_Door2_C"))
        (`self.K2_DestroyActor` _returnvalue_5)
        (bind _returnvalue_6 (`GameplayStatics.GetActorOfClass` "/Game/Blueprint/BP_NextFloor_1.BP_NextFloor_1_C"))
        (`|SpawnActorFromClass` "/Game/FirstPerson/Maps/Com_Room/Com_Door/Com_1_to_2.Com_1_to_2_C" (`KismetMathLibrary.Conv_VectorToTransform` (`self.K2_GetActorLocation` _returnvalue_6)) "Undefined" "MultiplyWithRoot" null null))
      (:`Computer_Room_2`
        (bind _outactors_4 (`GameplayStatics.GetAllActorsOfClass` "/Game/Blueprint/BP_worng_Door2.BP_worng_Door2_C"))
        (`self.K2_DestroyActor` _outactors_4)
        (bind _returnvalue_7 (`GameplayStatics.GetActorOfClass` "/Game/Blueprint/BP_NextFloor_1.BP_NextFloor_1_C"))
        (`|SpawnActorFromClass` "/Game/FirstPerson/Maps/Com_Room/Com_Door/Com_2_to_3.Com_2_to_3_C" (`KismetMathLibrary.Conv_VectorToTransform` (`self.K2_GetActorLocation` _returnvalue_7)) "Undefined" "MultiplyWithRoot" null null))
      (:`Computer_Room_3`
        (bind _outactors_5 (`GameplayStatics.GetAllActorsOfClass` "/Game/Blueprint/BP_worng_Door2.BP_worng_Door2_C"))
        (`self.K2_DestroyActor` _outactors_5)
        (bind _returnvalue_8 (`GameplayStatics.GetActorOfClass` "/Game/Blueprint/BP_NextFloor_1.BP_NextFloor_1_C"))
        (`|SpawnActorFromClass` "/Game/FirstPerson/Maps/Com_Room/Com_Door/Com_3_to_Lab.Com_3_to_Lab_C" (`KismetMathLibrary.Conv_VectorToTransform` (`self.K2_GetActorLocation` _returnvalue_8)) "Undefined" "MultiplyWithRoot" null null)))))

(fn `UserConstructionScript`)