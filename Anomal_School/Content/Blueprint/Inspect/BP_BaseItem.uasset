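; Base actor for world items that a character can inspect, with configurable mesh, name, scale and sound.
; The construction script sizes inner and outer spheres, places the interact icons, applies the mesh and shows the icons only when debugging.
; When inspection is enabled, OnInspect spawns a BP_InspectItem at a far-off location and passes it the mesh, name, inspection transform, character and itself for 2D sound playback.
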(event `/Game/Blueprint/Inspect/BPI-Interack.OnInspect`
  (params (Character :type "/Game/FirstPerson/Blueprints/BP_FirstPersonCharacter Object Reference"))
  (if (`self.Inspect?`)
    (bind _returnvalue (`|SpawnActorFromClass` "/Game/Blueprint/Inspect/BP_InspectItem.BP_InspectItem_C" (`KismetMathLibrary.MakeTransform` (100000.0 0.0 0.0)) "Undefined" "MultiplyWithRoot" null null))
    (`/Game/Blueprint/Inspect/BP_InspectItem.Set Inspect Rotaion` _returnvalue (`self.Item Inspection Rotation`))
    (`/Game/Blueprint/Inspect/BP_InspectItem.Set Inspect Scale` _returnvalue (`self.Item Inspection  Scale`))
    (`/Game/Blueprint/Inspect/BP_InspectItem.Set itemsound` _returnvalue self)
    (message `/Game/Blueprint/Inspect/BPI-Interack.Inspect` _returnvalue Character (`StaticMeshComponent.StaticMesh` (`self.StaticMesh`)) (`self.Item name`))
    (else
      (`KismetSystemLibrary.PrintString` "!!!"))))

(event `PlayItemSound`
  (`GameplayStatics.PlaySound2D` (`self.ItemSound`) 1.0 1.0 0.0 null null))

(fn `UserConstructionScript`
  (bind _staticmesh (`self.StaticMesh`))
  (`|ExecutionSequence`
    (:`then_0`
      (`SphereComponent.SetSphereRadius` (`self.InnerSphere_2`) (`self.InnersphereRadain`) true)
      (`SphereComponent.SetSphereRadius` (`self.OuterSphere_2`) (`self.OutersphereRadain`) true)
      (`SceneComponent.K2_SetRelativeLocation` (`self.InnerInteractIcon`) (`self.Icon Location`) false false)
      (`SceneComponent.K2_SetRelativeLocation` (`self.OuterInteractIcon`) (`self.Icon Location`) false false))
    (:`then_1`
      (`StaticMeshComponent.SetStaticMesh` (`self.StaticMesh`) (`self.Item Mesh`))
      (`SceneComponent.K2_SetWorldTransform` _staticmesh (`KismetMathLibrary.MakeTransform` (`SceneComponent.K2_GetComponentLocation` _staticmesh) (`SceneComponent.K2_GetComponentRotation` _staticmesh) (`self.Item Scale`)) false false))
    (:`then_2`
      (if (`self.Debugging?`)
        (`SceneComponent.SetVisibility` (`self.InnerInteractIcon`) true false)
        (`SceneComponent.SetVisibility` (`self.OuterInteractIcon`) true false)
        (else
          (`SceneComponent.SetVisibility` (`self.InnerInteractIcon`) false false)
          (`SceneComponent.SetVisibility` (`self.OuterInteractIcon`) false false))))))