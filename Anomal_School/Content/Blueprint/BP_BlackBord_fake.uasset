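; Placeholder blackboard actor that, once triggered, becomes the real blackboard and opens up the next floor.
; Either first-person character overlap with its Box or the IA_Interact input, which has no proximity check, runs the shared sequence.
; It spawns BP_BlackBord at its transform and destroys itself.
; It also removes all BP_worng_Door2 actors and spawns Lab_1_to_2 at the BP_NextFloor_1 actor's location.
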(event `self.Box.OnComponentBeginOverlap`
  (params (OverlappedComponent :type "PrimitiveComponent Object Reference") (OtherActor :type "Actor Object Reference") (OtherComp :type "PrimitiveComponent Object Reference") (OtherBodyIndex :type Integer) (bFromSweep :type Boolean) (SweepResult :type "HitResult Structure (by ref)"))
  (cast `/Game/FirstPerson/Blueprints/BP_FirstPersonCharacter` OtherActor)
  (`|SpawnActorFromClass` "/Game/Blueprint/BP_BlackBord.BP_BlackBord_C" (`self.GetTransform` self) "Undefined" "MultiplyWithRoot" null null :!label _label)
  (`self.K2_DestroyActor` self)
  (bind _outactors (`GameplayStatics.GetAllActorsOfClass` "/Game/Blueprint/BP_worng_Door2.BP_worng_Door2_C"))
  (`self.K2_DestroyActor` _outactors)
  (bind _returnvalue (`GameplayStatics.GetActorOfClass` "/Game/Blueprint/BP_NextFloor_1.BP_NextFloor_1_C"))
  (`|SpawnActorFromClass` "/Game/FirstPerson/Maps/science_room/Lab_Door/Lab_1_to_2.Lab_1_to_2_C" (`KismetMathLibrary.Conv_VectorToTransform` (`self.K2_GetActorLocation` _returnvalue)) "Undefined" "MultiplyWithRoot" null null))

(event `EnhancedInput|/Game/FirstPerson/Input/Actions/IA_Interact`
  (params (ActionValue :type Boolean) (ElapsedSeconds :type "Float (double-precision)") (TriggeredSeconds :type "Float (double-precision)") (InputAction :type "InputAction Object Reference" :default "/Game/FirstPerson/Input/Actions/IA_Interact.IA_Interact"))
  (:`Triggered`
    (goto _label)))

(fn `UserConstructionScript`)