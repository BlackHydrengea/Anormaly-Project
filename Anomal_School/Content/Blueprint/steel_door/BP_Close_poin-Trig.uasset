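; A one-shot trigger actor that closes a steel door when the player enters its box.
; On overlap by BP_FirstPersonCharacter, it spawns BP_SteelDoor at the location of the SD_Close_pion marker actor, found by class, and plays a metal slam sound there.
; The HasSpawnedDoor flag prevents repeat spawns.
; An unconnected fragment that would destroy the door never runs.
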(event `self.Box.OnComponentBeginOverlap`
  (params (OverlappedComponent :type "PrimitiveComponent Object Reference") (OtherActor :type "Actor Object Reference") (OtherComp :type "PrimitiveComponent Object Reference") (OtherBodyIndex :type Integer) (bFromSweep :type Boolean) (SweepResult :type "HitResult Structure (by ref)"))
  (if (not (`self.HasSpawnedDoor`))
    (cast `/Game/FirstPerson/Blueprints/BP_FirstPersonCharacter` OtherActor)
    (bind _returnvalue (`GameplayStatics.GetActorOfClass` "/Game/Blueprint/steel_door/SD_Close_pion.SD_Close_pion_C"))
    (bind _returnvalue_2 (`self.K2_GetActorLocation` _returnvalue))
    (`|SpawnActorFromClass` "/Game/Blueprint/steel_door/BP_SteelDoor.BP_SteelDoor_C" (`KismetMathLibrary.Conv_VectorToTransform` _returnvalue_2) "Undefined" "MultiplyWithRoot" null null)
    (`GameplayStatics.PlaySoundAtLocation` "/Game/Asset/Sound/metal-door-slam-172172.metal-door-slam-172172" _returnvalue_2 (struct) 1.0 1.0 0.0 null null null null)
    (set `self.HasSpawnedDoor` true)))

(fn `UserConstructionScript`)