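; BP_FallenTrigger is a one-shot trigger volume that spawns two Fallen actors when something overlaps its box.
; On overlap it waits a second, plays a sound at itself, then spawns BP_Fallen and BP_Fallen_Fall at the locations of the BP_spawn_Fallen and BP_spawn_Fallen2 marker actors found by class.
; The FAlled flag is set only after the delay and spawning, and the overlapping actor is not filtered.
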(event `self.Box.OnComponentBeginOverlap`
  (params (OverlappedComponent :type "PrimitiveComponent Object Reference") (OtherActor :type "Actor Object Reference") (OtherComp :type "PrimitiveComponent Object Reference") (OtherBodyIndex :type Integer) (bFromSweep :type Boolean) (SweepResult :type "HitResult Structure (by ref)"))
  (if (not (`self.FAlled`))
    (`KismetSystemLibrary.Delay` 1.0)
    (`GameplayStatics.PlaySoundAtLocation` "/Engine/VREditor/Sounds/UI/Floating_UI_Open-001.Floating_UI_Open-001" (`self.K2_GetActorLocation`) (struct) 1.0 1.0 0.0 null null null null)
    (bind _returnvalue (`GameplayStatics.GetActorOfClass` "/Game/Blueprint/Fallen/BP_spawn_Fallen.BP_spawn_Fallen_C"))
    (`|SpawnActorFromClass` "/Game/Blueprint/Fallen/BP_Fallen.BP_Fallen_C" (`KismetMathLibrary.Conv_VectorToTransform` (`self.K2_GetActorLocation` _returnvalue)) "Undefined" "MultiplyWithRoot" null null)
    (bind _returnvalue_2 (`GameplayStatics.GetActorOfClass` "/Game/Blueprint/Fallen/BP_spawn_Fallen-2.BP_spawn_Fallen-2_C"))
    (`|SpawnActorFromClass` "/Game/Blueprint/Fallen/BP_Fallen_Fall.BP_Fallen_Fall_C" (`KismetMathLibrary.Conv_VectorToTransform` (`self.K2_GetActorLocation` _returnvalue_2)) "Undefined" "MultiplyWithRoot" null null)
    (set `self.FAlled` true)))

(fn `UserConstructionScript`)