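; BP_Dialogue is a one-time trigger actor that opens the WD_UI_tutorial widget for the first-person player.
; Box end overlap and IA_Interact share one path that casts to BP_FirstPersonCharacter, checks HasPlayed, shows the widget and mouse cursor, and disables character input.
; Nothing live restores input.
; The indexed dialogue stepping through WD_Dialogue, hint sound and delayed widget cleanup are disconnected and never run.
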(event `self.Box.OnComponentEndOverlap`
  (params (OverlappedComponent :type "PrimitiveComponent Object Reference") (OtherActor :type "Actor Object Reference") (OtherComp :type "PrimitiveComponent Object Reference") (OtherBodyIndex :type Integer))
  (cast `/Game/FirstPerson/Blueprints/BP_FirstPersonCharacter` OtherActor :!label _label)
  (if (not (`self.HasPlayed`))
    (bind _returnvalue (`|CreateWidget` "/Game/UI/WD_UI_tutorial.WD_UI_tutorial_C"))
    (`UserWidget.AddToViewport` _returnvalue 0)
    (set `self.HasPlayed` true)
    (set `PlayerController.bShowMouseCursor` true (`GameplayStatics.GetPlayerController` 0))
    (`self.DisableInput` (`GameplayStatics.GetPlayerCharacter` 0) null)))

(event `EnhancedInput|/Game/FirstPerson/Input/Actions/IA_Interact`
  (params (ActionValue :type Boolean) (ElapsedSeconds :type "Float (double-precision)") (TriggeredSeconds :type "Float (double-precision)") (InputAction :type "InputAction Object Reference" :default "/Game/FirstPerson/Input/Actions/IA_Interact.IA_Interact"))
  (:`Triggered`
    (goto _label)))

(fn `UserConstructionScript`)